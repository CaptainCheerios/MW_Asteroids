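; Scene component that repeatedly spawns projectiles of a configurable class at its own world location and rotation while firing.
; StartShooting and StopShooting toggle the Firing flag, and Tick accumulates wait time, calling Fire once the interval has elapsed.
; BeginPlay converts the default rate of fire from rounds per minute to a seconds interval and primes the timer for an immediate first shot.
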(event Custom|Start%20Shooting
  (Variables|Default|SetbFiring true))

(event Custom|Stop%20Shooting
  (Variables|Default|SetbFiring false))

(event Custom|Fire
  (Variables|Default|SettimeWaitingToFire 0.0)
  (CallFunction|SpawnProjectile))

(event EventBeginPlay
  (Variables|Default|SetrateOfFire (Variables|Default|GetdefaultRateOfFire))
  (CallFunction|UpdateRateOfFire)
  (CallFunction|ResetFireDelay))

(event EventTick
  (params (DeltaSeconds :type Float%20%28single-precision%29))
  ;[1 1 1] Add time to the amount we've waited
  (Variables|Default|SettimeWaitingToFire (+ DeltaSeconds (Variables|Default|GettimeWaitingToFire)))
  (if (Variables|Default|GetbFiring)
    (if (<= (Variables|Default|GetfiringInterval) (Variables|Default|GettimeWaitingToFire))
      (CallFunction|Fire))))

(fn SpawnProjectile
  (Game|SpawnActorfromClass (Variables|Default|GetprojectileClass) (Math|Transform|MakeTransform (Transformation|GetWorldLocation) (Transformation|GetWorldRotation) "1,1,1") "AlwaysSpawn" 0 0))

(fn UpdateRateOfFire
  (Variables|Default|SetfiringInterval (/ 1.0 (/ (Variables|Default|GetrateOfFire) 6e+01))))

(fn ResetFireDelay
  (Variables|Default|SettimeWaitingToFire (Variables|Default|GetfiringInterval)))