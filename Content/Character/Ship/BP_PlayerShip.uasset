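; Player ship Blueprint that holds steering input and the math for a clamped rotation speed.
; RotateRight and RotateLeft input events store their steering value as SteeringDirection.
; HandleSteering multiplies an FInterpTo drag result by change speed and direction, adds it to the current speed, and clamps it symmetrically.
; The event graph is empty; nothing here calls HandleSteering or applies the speed to the actor.
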(event EventBeginPlay)

(event Collision|EventActorBeginOverlap
  (params (OtherActor :type Actor%20Object%20Reference)))

(event EventTick
  (params (DeltaSeconds :type Float%20%28single-precision%29)))

(event Custom|Rotate%20Right
  (params (Steering :type Float%20%28single-precision%29))
  (Variables|Movement|Rotation|SetSteeringDirection Steering))

(event Custom|Rotate%20Left
  (params (Steering :type Float%20%28single-precision%29))
  (Variables|Movement|Rotation|SetSteeringDirection Steering))

(fn ConstructionScript)

(fn HandleSteering
  (params (DeltaTime :type Float%20%28single-precision%29))
  (Variables|Movement|Rotation|SetCurrentRotationSpeed (Math|Float|Clamp(Float) (+ (* (Math|Interpolation|FInterpTo (Variables|Movement|Rotation|GetCurrentRotationSpeed) 0.0 DeltaTime (Variables|Movement|Rotation|GetRotationDrag)) (Variables|Movement|Rotation|GetRotationChangeSpeed) (Variables|Movement|Rotation|GetSteeringDirection)) (Variables|Movement|Rotation|GetCurrentRotationSpeed)) (* -1.0 (Variables|Movement|Rotation|GetMaxRotationSpeed)) (Variables|Movement|Rotation|GetMaxRotationSpeed))))