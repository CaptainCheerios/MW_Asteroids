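; Destructible physics asteroid that can drift on a random yaw heading and breaks into smaller asteroids when damage depletes its health.
; Construction fits the collision box to the mesh bounds.
; On death it picks a random ChildAsteroidsToSpawn entry and launches up to twelve chunks along unique 30-degree yaw slots with a random offset.
; Explosion effects are an empty stub, and an older child-actor hide-and-detach approach remains, mostly unused.
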(event Custom|Explode
  (CallFunction|SpawnExplosionEffects)
  (CallFunction|SpawnAsteroidChunks)
  (Actor|DestroyActor))

(event Custom|Activate%20Children)

(event Custom|Destroy%20Self
  ;[1 1 1] Old code was used for my prior attempt to build asteroids that could be better designed visually
  (CallFunction|SpawnExplosionEffects)
  (Actor|DestroyActor))

(event Custom|Deparent_Activate
  (Collision|SetActorEnableCollision true)
  (Transformation|DetachFromActor self "KeepWorld" "KeepWorld" "KeepWorld")
  (Physics|SetSimulatePhysics (Variables|Default|GetBox) true)
  (Collision|SetCollisionEnabled (Variables|Default|GetBox) "QueryAndPhysics")
  (Rendering|SetVisibility (Variables|Default|GetMeshComponent) true false))

(event Custom|ChildDestroyed
  (if (== (Utilities|Array|Length (Actor|GetAllChildActors true)) 0)
    (Actor|DestroyActor)))

(event EventBeginPlay
  (if (Variables|Default|GetbRandomVelocity)
    (CallFunction|AddRandomAcceleration)))

(event Collision|EventActorBeginOverlap
  (params (OtherActor :type Actor%20Object%20Reference)))

(event EventTick
  (params (DeltaSeconds :type Float%20%28single-precision%29)))

(event Game|Damage|EventAnyDamage
  (params (Damage :type Float%20%28single-precision%29) (DamageType :type Damage%20Type%20Object%20Reference) (InstigatedBy :type Controller%20Object%20Reference) (DamageCauser :type Actor%20Object%20Reference))
  (CallFunction|TakeDamage Damage))

(event EventDestroyed
  (Default|CallNotifyParentChildWasDestroyed))

(fn ConstructionScript
  ;[1 1 1] No Longer Used
  (CallFunction|UpdateCollisionBox))

(fn TakeDamage
  (params (Damage :type Float%20%28single-precision%29))
  (bind _output_get (Variables|Default|Sethealth (- (Variables|Default|Gethealth) Damage)))
  (if (<= _output_get 0.0)
    (CallFunction|Explode)))

(fn SpawnExplosionEffects)

(fn GetChildAsteroids
  (Utilities|Array|Clear (Variables|Default|GetchildAsteroids))
  (for _array_element (Actor|GetAllChildActors false)
    (bind _asbp_asteroid (Utilities|Casting|CastToBP_Asteroid _array_element))
    (Utilities|Array|Add (Variables|Default|GetchildAsteroids) _asbp_asteroid)
    (EventDispatchers|BindEventtoNotifyParentChildWasDestroyed _asbp_asteroid (EventDispatchers|CreateEvent :!event Custom|ChildDestroyed))))

(fn HideifAChild
  ;[1 1 1] If we are a child we don't want to be visible
  (Utilities|IsValid (Actor|GetParentActor)
    (:Is%20Valid
      (CallFunction|Deactivate))))

(fn UpdateCollisionBox
  (Components|Box|SetBoxExtent (Variables|Default|GetBox) (.BoxExtent (Collision|GetComponentBounds (Variables|Default|GetMeshComponent))) true))

(fn Deactivate
  (Collision|SetActorEnableCollision false)
  (Collision|SetCollisionEnabled (Variables|Default|GetBox) "NoCollision")
  (Physics|SetSimulatePhysics (Variables|Default|GetBox) false)
  (Rendering|SetVisibility (Variables|Default|GetMeshComponent) false false))

(fn SpawnAsteroidChunks
  ;[1 1 1] Comment
  (if (> (Utilities|Array|Length (Variables|Default|GetchildAsteroidsToSpawn)) 0)
    (bind _result (Math|Integer|DecrementInt (Math|Random|RandomIntegerinRange 1 (Utilities|Array|Length (Variables|Default|GetchildAsteroidsToSpawn))))
      (:%20%20
        (LocalVariables|SetasteroidsToSpawn (Math|Integer|Clamp(Integer) (.Count (Utilities|Struct|BreakStruct_AsteroidChunkSpawn (Utilities|Array|Get(acopy) (Variables|Default|GetchildAsteroidsToSpawn) _result))) 1 12))
        (Utilities|FlowControl|Sequence
          (:then_0
            ;;[1 1 1] We want to get Unique set of positions to spawn at, so keep adding (not effecient but we only want max 12)
            (while (< (Utilities|Set|Length (LocalVariables|Getpositions)) (LocalVariables|GetasteroidsToSpawn))
              (Utilities|Set|Add (LocalVariables|Getpositions) (Math|Random|RandomIntegerinRange 0 11))))
          (:then_1
            ;;[1 1 1] Create an offset so we give it a bit more of a twist and it doesn't look like 1/12 directions
            (LocalVariables|SetOffset (Math|Random|RandomIntegerinRange 0 30)))
          (:then_2
            (bind _result_2 (Utilities|Set|ToArray (LocalVariables|Getpositions)))
            (for _array_element _result_2
              (bind _returnvalue (Game|SpawnActorfromClass (.AsteroidToSpawn (Utilities|Struct|BreakStruct_AsteroidChunkSpawn (Utilities|Array|Get(acopy) (Variables|Default|GetchildAsteroidsToSpawn) _result))) (Math|Transform|MakeTransform (Transformation|GetActorLocation) (Transformation|GetActorRotation) "1,1,1") "AlwaysSpawn" 0 false 0))
              ;;[1 1 1] Sometimes it gets blown up before it even gets to add force
              (Utilities|IsValid _returnvalue
                (:Is%20Valid
                  (Physics|AddForce (Variables|BP_Asteroid_C|GetBox _returnvalue) (* (Math|Vector|GetForwardVector (Math|Rotator|MakeRotator 0.0 0.0 (Math|Conversions|ToFloat(Integer) (+ (* _array_element 30) (LocalVariables|GetOffset))))) (Math|Random|RandomFloatinRange (Variables|Default|GetminVelocity) (Variables|Default|GetmaxVelocity))) "None" true))))))))
    (else
      (return))))

(fn AddRandomAcceleration
  (Physics|AddForce (Variables|Default|GetBox) (* (Math|Vector|GetForwardVector (Math|Rotator|MakeRotator 0.0 0.0 (Math|Random|RandomFloatinRange 0.0 3.6e+02))) (Math|Random|RandomFloatinRange (Variables|Default|GetminVelocity) (Variables|Default|GetmaxVelocity))) "None" true))