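; Unfinished asteroid spawner meant to place asteroids in one of several spawn areas, favoring areas free of the player ship.
; FindBestSpawn samples a random area, returning it if empty, otherwise recording asteroid counts of player-free areas and returning the lowest recorded.
; That fallback return sits inside the loop, so only one area is sampled per call.
; SpawnAsteroid and InitialSpawn are empty, and the graph linking selection to spawning never runs.
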(event Custom|Initial%20Spawn)

(event EventBeginPlay)

(event Collision|EventActorBeginOverlap
  (params (OtherActor :type Actor%20Object%20Reference)))

(event EventTick
  (params (DeltaSeconds :type Float%20%28single-precision%29)))

(fn ConstructionScript)

(fn CheckforPlayer
  (params (SpawnArea :type Actor%20Object%20Reference))
  (return (> (Utilities|Array|Length (Collision|GetOverlappingActors SpawnArea "/Game/Pawns/Ship/BP_PlayerShip.BP_PlayerShip_C" :!class /Script/Engine.Actor)) 0)))

(fn GetTotalAsteroidsinVolume
  (params (SpawnArea :type Actor%20Object%20Reference))
  (return (Utilities|Array|Length (Collision|GetOverlappingActors SpawnArea "/Script/MW_Asteroids.Asteroid" :!class /Script/Engine.Actor))))

(fn FindBestSpawn
  (bind _spawnareas (Variables|Default|GetspawnAreas))
  (bind _returnvalue (Utilities|Array|Length _spawnareas))
  (bind _returnvalue_2 (- _returnvalue 1))
  (Utilities|FlowControl|ForLoopwithBreak 0 _returnvalue_2
    (:LoopBody
      (LocalVariables|SetcurrentIndex (Math|Random|RandomIntegerinRange 0 _returnvalue_2))
      (Utilities|FlowControl|Sequence
        (:then_0
          (bind _returnvalue_3 (CallFunction|CheckforPlayer (Utilities|Array|Get(acopy) (Variables|Default|GetspawnAreas) (LocalVariables|GetcurrentIndex))))
          (if _returnvalue_3
            (LocalVariables|SetspawnWithPlayer (LocalVariables|GetcurrentIndex))
            (else
              (bind _returnvalue1 (CallFunction|GetTotalAsteroidsinVolume (Utilities|Array|Get(acopy) (Variables|Default|GetspawnAreas) (LocalVariables|GetcurrentIndex))))
              (if (== _returnvalue1 0)
                (return (LocalVariables|GetcurrentIndex))
                (else
                  (Utilities|Map|Add (LocalVariables|GetasteroidCount) (LocalVariables|GetcurrentIndex) _returnvalue1))))))
        (:then_1
          (bind _keys (Utilities|Map|Keys (LocalVariables|GetasteroidCount)))
          (LocalVariables|SetindexOfCurrentBest (Utilities|Array|Get(acopy) _keys))
          (LocalVariables|SetlowestAsteroidCount (.Value (Utilities|Map|Find (LocalVariables|GetasteroidCount) (Utilities|Array|Get(acopy) _keys))))
          (for _array_element _keys
            (if (< (.Value (Utilities|Map|Find (LocalVariables|GetasteroidCount) _array_element)) (LocalVariables|GetlowestAsteroidCount))
              (LocalVariables|SetindexOfCurrentBest _array_element)
              (LocalVariables|SetlowestAsteroidCount (.Value (Utilities|Map|Find (LocalVariables|GetasteroidCount) _array_element)))))
          (return (LocalVariables|GetindexOfCurrentBest)))))))

(fn SpawnAsteroid
  (params (SpawnArea :type Trigger%20Volume%20Object%20Reference)))