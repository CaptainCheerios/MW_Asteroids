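; BP_Asteroid_WB_A is a whitebox asteroid Blueprint that relies on its parent class for its behavior.
; Tick calls the parent, then prints the collision-enabled state of the Box and MeshComponent every frame with zero duration, as a live debug readout.
; The construction script only calls the parent, and the BeginPlay and overlap events are disabled stubs.
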(event EventBeginPlay
  (|CallParentFunction) ; This node is disabled and will not be called.\nDrag off pins to build functionality.
)

(event Collision|EventActorBeginOverlap
  (params (OtherActor :type Actor%20Object%20Reference))
  (|CallParentFunction OtherActor) ; This node is disabled and will not be called.\nDrag off pins to build functionality.
)

(event EventTick
  (params (DeltaSeconds :type Float%20%28single-precision%29))
  (|CallParentFunction DeltaSeconds)
  (Development|PrintText (Utilities|Text|FormatText "BoxCollision:{BC} 
MeshComponent:{MC}" (Utilities|String|EnumtoString (Collision|GetCollisionEnabled (Variables|Default|GetBox))) (Utilities|String|EnumtoString (Collision|GetCollisionEnabled (Variables|Default|GetMeshComponent)))) true true "(R=0.000000,G=0.660000,B=1.000000,A=1.000000)" 0.0))

(fn ConstructionScript
  (|CallParentFunction))